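; BP_P38 is a player-controlled P-38 aircraft that handles rotation, rocket fire and boost through Enhanced Input.
; Rotate input applies frame-time-scaled local roll and pitch.
; Fire spawns BP_Rocket at the left or right arrow component, using a FlipFlop to alternate sides.
; Boost raises BoostValue when triggered and lowers it only on cancel; nothing in this graph reads that value.
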(event Input|EnhancedActionEvents|EnhancedInputActionIA_Rotate
  (params (ActionValue :type Vector%202D%20Structure) (ElapsedSeconds :type Float%20%28double-precision%29) (TriggeredSeconds :type Float%20%28double-precision%29) (InputAction :type Input%20Action%20Object%20Reference :default "/Game/Blueprints/Input/IA_Rotate.IA_Rotate"))
  (bind _returnvalue (Utilities|Time|GetWorldDeltaSeconds))
  (Transformation|AddActorLocalRotation (Math|Rotator|MakeRotator (* (.x ActionValue) _returnvalue 6e+01) 0.0 0.0) false false)
  (Transformation|AddActorLocalRotation (Math|Rotator|MakeRotator 0.0 (* (.y ActionValue) _returnvalue 6e+01) 0.0) false false))

(event Input|EnhancedActionEvents|EnhancedInputActionIA_Fire
  (params (ActionValue :type Boolean) (ElapsedSeconds :type Float%20%28double-precision%29) (TriggeredSeconds :type Float%20%28double-precision%29) (InputAction :type Input%20Action%20Object%20Reference :default "/Game/Blueprints/Input/IA_Fire.IA_Fire"))
  (:Triggered
    (bind _isa (Utilities|FlowControl|FlipFlop)
      (:A
        _)
      (:B
        _))
    (Game|SpawnActorfromClass "/Game/Blueprints/CPP/BP_Rocket.BP_Rocket_C" (Transformation|GetWorldTransform (select _isa (Variables|Default|GetLeftArrow) (Variables|Default|GetRightArrow))) "AdjustIfPossibleButAlwaysSpawn" "MultiplyWithRoot" 0 0)))

(event Input|EnhancedActionEvents|EnhancedInputActionIA_Boost
  (params (ActionValue :type Boolean) (ElapsedSeconds :type Float%20%28double-precision%29) (TriggeredSeconds :type Float%20%28double-precision%29) (InputAction :type Input%20Action%20Object%20Reference :default "/Game/Blueprints/Input/IA_Boost.IA_Boost"))
  (:Triggered
    (Variables|Default|SetBoostValue 1.0))
  (:Canceled
    (Variables|Default|SetBoostValue 0.5)))

(fn ConstructionScript)